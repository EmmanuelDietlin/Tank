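; Projectile actor that damages tanks and ricochets off whatever else it strikes.
; On a sphere hit, it calls TakeHit on a Tank and destroys itself, with debug prints left in.
; It decrements Bounces without checking it, then reflects its yaw off the hit normal, using dot products to pick turn direction and angle while keeping pitch and roll.
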(event `self.Sphere.OnComponentHit`
  (params (HitComponent :type "PrimitiveComponent Object Reference") (OtherActor :type "Actor Object Reference") (OtherComp :type "PrimitiveComponent Object Reference") (NormalImpulse :type "Vector Structure") (Hit :type "HitResult Structure (by ref)"))
  (bind _roll (.roll (`self.K2_GetActorRotation`)))
  (bind _pitch (.pitch (`self.K2_GetActorRotation`)))
  (bind _yaw (.yaw (`self.K2_GetActorRotation`)))
  (bind _returnvalue (`KismetMathLibrary.Normal` (`.Normal` (`GameplayStatics.BreakHitResult` Hit))))
  (bind _returnvalue_2 (`KismetMathLibrary.Normal` (`self.GetActorForwardVector`)))
  (bind _returnvalue_3 (* (- 90.0 (`KismetMathLibrary.DegAcos` (`KismetMathLibrary.Dot_VectorVector` _returnvalue_2 _returnvalue))) 2.0))
  (bind _astank (cast `Tank` OtherActor)
    (:`then`
      (`KismetSystemLibrary.PrintString` "Hello")
      (`Tank.TakeHit` _astank)
      (`self.K2_DestroyActor`))
    (:`CastFailed`
      (`KismetSystemLibrary.PrintString` "aaaaa")))
  (set `self.Bounces` (- (`self.Bounces`) 1))
  (`/Engine/EditorBlueprintResources/StandardMacros.CompareFloat` (`KismetMathLibrary.Dot_VectorVector` _returnvalue_2 (`KismetMathLibrary.RotateAngleAxis` _returnvalue 90.0 (0.0 0.0 1.0)))
    (:`>`
      (`self.K2_SetActorRotation` (`KismetMathLibrary.MakeRotator` _roll _pitch (+ _returnvalue_3 _yaw)) :!label _label))
    (:`==`
      (goto _label))
    (:`<`
      (`self.K2_SetActorRotation` (`KismetMathLibrary.MakeRotator` _roll _pitch (+ (* _returnvalue_3 -1.0) _yaw))))))

(fn `UserConstructionScript`)