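; Player controller for the tank campaign mode that carries the player's name and color and manages that player's screens.
; Setup can read the name from the TankSave slot, caches the campaign game mode, and a separate event applies name and color to the controlled tank.
; Pause input toggles pause through the game mode and game instance, while other events lazily create HUD, victory, defeat, transition and loading widgets.
; Individual score handling is unfinished.
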(event `InitialSetup`
  (params (PlayerColor :type "MaterialInterface Object Reference") (DisplayName :type Boolean))
  (bind _returnvalue (`GameplayStatics.LoadGameFromSlot` "TankSave"))
  (bind _astank_save_game (cast `TankSaveGame` _returnvalue))
  (if DisplayName
    (bind _playerinfos_playername (break `PlayerInfos` (`TankSaveGame.PlayerInfos` _astank_save_game)))
    (bind _output_get (set `self.PlayerName` _playerinfos_playername)))
  (bind _output_get_2 (set `self.PlayerColor` PlayerColor))
  (`self.CallUpdate` _output_get_2 _output_get))

(event `CallUpdate`
  (params (PlayerColor :type "MaterialInterface Object Reference") (PlayerName :type String))
  (set `self.PlayerName` PlayerName)
  (set `self.PlayerColor` PlayerColor)
  (bind _ascampaign_tank_game_mode (cast `/Game/Tank/Gameplay/CampaignTankGameMode` (`GameplayStatics.GetGameMode`)))
  (set `self.GameMode` _ascampaign_tank_game_mode))

(event `self.ReceiveBeginPlay`)

(event `EnhancedInput|/Game/Tank/Inputs/Tank_Pause`
  (params (ActionValue :type Boolean) (ElapsedSeconds :type "Float (double-precision)") (TriggeredSeconds :type "Float (double-precision)") (InputAction :type "InputAction Object Reference" :default "/Game/Tank/Inputs/Tank_Pause.Tank_Pause"))
  (:`Triggered`
    (bind _asbp_player_tank (cast `/Game/Tank/Blueprints/Tanks/BP_PlayerTank` (`self.K2_GetPawn`)))
    (bind _asbp_player_tank_2 (cast `/Game/Tank/Blueprints/Tanks/BP_PlayerTank` (`self.K2_GetPawn`)))
    (bind _ispaused (`Tank.IsPaused` _asbp_player_tank))
    (`/Game/Tank/Gameplay/CampaignTankGameMode.TogglePausePlayer` (`self.GameMode`) (not _ispaused) _asbp_player_tank_2)
    (bind _asbp_tank_game_instance (cast `/Game/Tank/Blueprints/Game/BP_TankGameInstance` (`GameplayStatics.GetGameInstance`)))
    (if _ispaused
      (`/Game/Tank/Blueprints/Game/BP_TankGameInstance.ShowPauseScreen` _asbp_tank_game_instance)
      (else
        (`/Game/Tank/Blueprints/Game/BP_TankGameInstance.RemovePauseScreen` _asbp_tank_game_instance)))))

(event `SetupDefeatScreen`
  (`/Engine/EditorBlueprintResources/StandardMacros.IsValid` (`self.DefeatScreen`)
    (:`Is Valid`
      _)
    (:`Is Not Valid`
      (bind _returnvalue (`|CreateWidget` "/Game/Tank/UI/WBP_DefeatScreen_.WBP_DefeatScreen__C"))
      (set `self.DefeatScreen` _returnvalue)))
  (`UserWidget.AddToViewport` (`self.DefeatScreen`) 0))

(event `ShowVictoryScreen`
  (`/Engine/EditorBlueprintResources/StandardMacros.IsValid` (`self.VictoryScreen`)
    (:`Is Valid`
      _)
    (:`Is Not Valid`
      (bind _returnvalue (`|CreateWidget` "/Game/Tank/UI/WBP_VictoryScreen_.WBP_VictoryScreen__C"))
      (set `self.VictoryScreen` _returnvalue)))
  (`UserWidget.AddToViewport` (`self.VictoryScreen`) 0))

(event `SetupHUD`
  (`/Engine/EditorBlueprintResources/StandardMacros.IsValid` (`self.HUD`)
    (:`Is Valid`
      _)
    (:`Is Not Valid`
      (bind _returnvalue (`|CreateWidget` "/Game/Tank/UI/WBP_CampaignHUD.WBP_CampaignHUD_C"))
      (set `self.HUD` _returnvalue)))
  (`UserWidget.AddToViewport` (`self.HUD`) 0))

(event `SetPlayerTankNameAndColor`
  (bind _asbp_player_tank (cast `/Game/Tank/Blueprints/Tanks/BP_PlayerTank` (`self.K2_GetPawn`)))
  (`/Game/Tank/Blueprints/Tanks/BP_PlayerTank.SetPlayerNameAndColor` _asbp_player_tank (`self.PlayerName`) (`self.PlayerColor`)))

(event `SetupTransitionScreen`
  (`/Engine/EditorBlueprintResources/StandardMacros.IsValid` (`self.TransitionScreen`)
    (:`Is Valid`
      _)
    (:`Is Not Valid`
      (bind _returnvalue (`|CreateWidget` "/Game/Tank/UI/WBP_TransitionScreen.WBP_TransitionScreen_C"))
      (set `self.TransitionScreen` _returnvalue)))
  (`UserWidget.AddToViewport` (`self.TransitionScreen`) 0))

(event `SetupLoadingScreen`
  (`/Engine/EditorBlueprintResources/StandardMacros.IsValid` (`self.LoadingScreen`)
    (:`Is Valid`
      _)
    (:`Is Not Valid`
      (bind _returnvalue (`|CreateWidget` "/Game/Tank/UI/WBP_LoadingScreen.WBP_LoadingScreen_C"))
      (set `self.LoadingScreen` _returnvalue)))
  (`UserWidget.AddToViewport` (`self.LoadingScreen`) 0))

(event `BeginPlay`
  (bind _ascampaign_tank_game_mode (cast `/Game/Tank/Gameplay/CampaignTankGameMode` (`GameplayStatics.GetGameMode`)))
  (bind _asbp_player_tank (cast `/Game/Tank/Blueprints/Tanks/BP_PlayerTank` (`self.K2_GetPawn`)))
  (`/Game/Tank/Gameplay/CampaignTankGameMode.TogglePausePlayer` _ascampaign_tank_game_mode false _asbp_player_tank))

(event `SetIndividualScore`
  ;[1 1 1] TODO : à finir score individuel en mode campagne plusieurs joueurs
  (bind _asbp_tank_game_instance (cast `/Game/Tank/Blueprints/Game/BP_TankGameInstance` (`GameplayStatics.GetGameInstance`)))
  (set `/Game/Tank/Blueprints/Game/BP_TankGameInstance.IndividualScore` (`KismetMathLibrary.FTrunc` (`PlayerState.Score` (`self.PlayerState`))) _asbp_tank_game_instance))

(event `GetIndividualScore`
  ;[1 1 1] TODO : à finir score individuel en mode campagne plusieurs joueurs
  (cast `/Game/Tank/Blueprints/Game/BP_TankGameInstance` (`GameplayStatics.GetGameInstance`)))

(fn `UserConstructionScript`)