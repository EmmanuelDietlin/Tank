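; Player controller for the tank Versus mode, managing a player's name, color, lives, score and UI screens.
; Setup loads the name from the TankSave slot and registers player info with VersusTankGameMode.
; Life and score changes update the HUD and game mode, which also receives pause and start requests.
; On possession, the server makes the tank temporarily invincible for a duration set by the mode parameters.
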(event `self.ReceiveBeginPlay`)

(event `InitialSetup`
  (params (PlayerColor :type "MaterialInterface Object Reference") (Id :type Integer) (VersusModeParams :type "VersusGameData Structure"))
  (bind _output_get (set `self.PlayerColor` PlayerColor))
  (bind _output_get_2 (set `self.Versus Mode Params` VersusModeParams))
  (`self.SetGameInstance`)
  (bind _returnvalue (`GameplayStatics.DoesSaveGameExist` "TankSave"))
  (if _returnvalue
    (bind _returnvalue_2 (`GameplayStatics.LoadGameFromSlot` "TankSave"))
    (bind _astank_save_game (cast `TankSaveGame` _returnvalue_2))
    (bind _playerinfos_playername (break `PlayerInfos` (`TankSaveGame.PlayerInfos` _astank_save_game)))
    (bind _output_get_3 (set `self.PlayerInfos` (make `VersusPlayerInfos` Id _playerinfos_playername 0 (`.Lives` (break `VersusGameData` _output_get_2)))))
    (`self.CallUpdate` _output_get_3 _output_get _output_get_2)))

(event `CallUpdate`
  (params (`Player Infos` :type "VersusPlayerInfos Structure") (PlayerColor :type "MaterialInterface Object Reference") (VersusModeParams :type "VersusGameData Structure"))
  (set `self.Versus Mode Params` VersusModeParams)
  (set `self.PlayerInfos` `Player Infos`)
  (set `self.PlayerColor` PlayerColor)
  (bind _asversus_tank_game_mode (cast `/Game/Tank/Gameplay/VersusTankGameMode` (`GameplayStatics.GetGameMode`)))
  (`/Game/Tank/Gameplay/VersusTankGameMode.UpdatePlayerInfos` _asversus_tank_game_mode (`self.PlayerInfos`)))

(event `self.ReceivePossess`
  (params (PossessedPawn :type "Pawn Object Reference"))
  (bind (_versus_mode_params_versusmodetype _versus_mode_params_lives _versus_mode_params_timerseconds _versus_mode_params_invicibilityduration) (break `VersusGameData` (`self.Versus Mode Params`)))
  (if (`KismetSystemLibrary.IsServer`)
    (bind _asbp_player_tank (cast `/Game/Tank/Blueprints/Tanks/BP_PlayerTank` PossessedPawn))
    (set `Tank.CanBeDestroyed` false _asbp_player_tank)
    (`KismetSystemLibrary.Delay` _versus_mode_params_invicibilityduration)
    (set `Tank.CanBeDestroyed` true _asbp_player_tank)))

(event `SetupVersusHUD`
  (params (VersusModeParams :type "VersusPlayerInfos Structure"))
  (`/Engine/EditorBlueprintResources/StandardMacros.IsValid` (`self.HUD`)
    (:`Is Valid`
      _)
    (:`Is Not Valid`
      (bind _returnvalue (`|CreateWidget` "/Game/Tank/UI/WBP_VersusHUD.WBP_VersusHUD_C" null (`self.Versus Mode Params`)))
      (set `self.HUD` _returnvalue)))
  (`UserWidget.AddToViewport` (`self.HUD`) 0))

(event `SetupPauseScreen`
  (`/Engine/EditorBlueprintResources/StandardMacros.IsValid` (`self.PauseScreen`)
    (:`Is Valid`
      _)
    (:`Is Not Valid`
      (bind _returnvalue (`|CreateWidget` "/Game/Tank/UI/WBP_PauseScreen.WBP_PauseScreen_C"))
      (set `self.PauseScreen` _returnvalue)))
  (`UserWidget.AddToViewport` (`self.PauseScreen`) 0))

(event `SetupLoadingScreen`
  (`/Engine/EditorBlueprintResources/StandardMacros.IsValid` (`self.LoadingScreen`)
    (:`Is Valid`
      _)
    (:`Is Not Valid`
      (bind _returnvalue (`|CreateWidget` "/Game/Tank/UI/WBP_LoadingScreen.WBP_LoadingScreen_C"))
      (set `self.LoadingScreen` _returnvalue)))
  (`UserWidget.AddToViewport` (`self.LoadingScreen`) 0))

(event `RemovePauseScreen`
  (`Widget.RemoveFromParent` (`self.PauseScreen`)))

(event `SetupVersusStartScreen`
  (`/Engine/EditorBlueprintResources/StandardMacros.IsValid` (`self.VersusStart`)
    (:`Is Valid`
      _)
    (:`Is Not Valid`
      (bind _returnvalue (`|CreateWidget` "/Game/Tank/UI/WBP_VersusStartScreen.WBP_VersusStartScreen_C"))
      (set `self.VersusStart` _returnvalue)))
  (`UserWidget.AddToViewport` (`self.VersusStart`) 0))

(event `LoseLife`
  (bind _playerinfos (`self.PlayerInfos`))
  (bind _structout (setmembers `VersusPlayerInfos` :`StructRef` _playerinfos :`Lives` (- (`.Lives` (break `VersusPlayerInfos` _playerinfos)) 1)))
  (`self.UpdateLife` _structout)
  (bind _asversus_tank_game_mode (cast `/Game/Tank/Gameplay/VersusTankGameMode` (`GameplayStatics.GetGameMode`)))
  (`/Game/Tank/Gameplay/VersusTankGameMode.UpdatePlayerInfos` _asversus_tank_game_mode (`self.PlayerInfos`)))

(event `SetupEndScreen`
  (params (VersusPlayerInfos :type "Array of VersusPlayerInfos Structure"))
  (`/Engine/EditorBlueprintResources/StandardMacros.IsValid` (`self.EndScreen`)
    (:`Is Valid`
      _)
    (:`Is Not Valid`
      (bind _returnvalue (`|CreateWidget` "/Game/Tank/UI/WBP_VersusEndScreen.WBP_VersusEndScreen_C" null VersusPlayerInfos))
      (set `self.EndScreen` _returnvalue)))
  (`UserWidget.AddToViewport` (`self.EndScreen`) 0))

(event `UpdateLife`
  (params (PlayerInfos :type "VersusPlayerInfos Structure"))
  (`/Game/Tank/UI/WBP_VersusHUD.UpdateLives` (`self.HUD`) PlayerInfos_Lives))

(event `AddScore`
  (params (Points :type Integer))
  (bind _playerinfos (`self.PlayerInfos`))
  (bind _structout (setmembers `VersusPlayerInfos` :`StructRef` _playerinfos :`Score` (+ (`.Score` (break `VersusPlayerInfos` _playerinfos)) Points)))
  (`self.UpdateScore` _structout)
  (bind _asversus_tank_game_mode (cast `/Game/Tank/Gameplay/VersusTankGameMode` (`GameplayStatics.GetGameMode`)))
  (`/Game/Tank/Gameplay/VersusTankGameMode.UpdatePlayerInfos` _asversus_tank_game_mode (`self.PlayerInfos`)))

(event `UpdateScore`
  (params (PlayerInfos :type "VersusPlayerInfos Structure"))
  (`/Game/Tank/UI/WBP_VersusHUD.UpdateScore` (`self.HUD`) PlayerInfos_Score))

(event `UpdateTimer`
  (params (Timer :type "Float (double-precision)"))
  (bind _hud (`self.HUD`))
  (`/Engine/EditorBlueprintResources/StandardMacros.IsValid` _hud
    (:`Is Valid`
      (`/Game/Tank/UI/WBP_VersusHUD.UpdateTimer` _hud (`KismetMathLibrary.Round` Timer)))))

(event `TogglePausePlayer`
  (params (Pause :type Boolean))
  (bind _returnvalue (`self.K2_GetPawn`))
  (`/Engine/EditorBlueprintResources/StandardMacros.IsValid` _returnvalue
    (:`Is Valid`
      (bind _asbp_player_tank (cast `/Game/Tank/Blueprints/Tanks/BP_PlayerTank` _returnvalue))
      (`Tank.TogglePause` _asbp_player_tank Pause))))

(event `EnhancedInput|/Game/Tank/Inputs/Tank_Pause`
  (params (ActionValue :type Boolean) (ElapsedSeconds :type "Float (double-precision)") (TriggeredSeconds :type "Float (double-precision)") (InputAction :type "InputAction Object Reference" :default "/Game/Tank/Inputs/Tank_Pause.Tank_Pause"))
  (:`Triggered`
    (bind _asbp_player_tank (cast `/Game/Tank/Blueprints/Tanks/BP_PlayerTank` (`self.K2_GetPawn`)))
    (bind _asversus_tank_game_mode (cast `/Game/Tank/Gameplay/VersusTankGameMode` (`GameplayStatics.GetGameMode`)))
    (bind _ispaused (`Tank.IsPaused` _asbp_player_tank))
    (`/Game/Tank/Gameplay/VersusTankGameMode.TogglePlayerPause` _asversus_tank_game_mode self (not _ispaused))
    (if _ispaused
      (`self.SetupPauseScreen`)
      (else
        (`self.RemovePauseScreen`)))))

(event `SetPlayerTankNameAndColor`
  (bind (_playerinfos_id _playerinfos_playername) (break `VersusPlayerInfos` (`self.PlayerInfos`)))
  (bind _asbp_player_tank (cast `/Game/Tank/Blueprints/Tanks/BP_PlayerTank` (`self.K2_GetPawn`)))
  (`/Game/Tank/Blueprints/Tanks/BP_PlayerTank.SetPlayerNameAndColor` _asbp_player_tank _playerinfos_playername (`self.PlayerColor`)))

(event `StartGame`
  (bind _asversus_tank_game_mode (cast `/Game/Tank/Gameplay/VersusTankGameMode` (`GameplayStatics.GetGameMode`)))
  (`/Game/Tank/Gameplay/VersusTankGameMode.TogglePlayerPause` _asversus_tank_game_mode self false))

(fn `SetGameInstance`
  (bind _asbp_tank_game_instance (cast `/Game/Tank/Blueprints/Game/BP_TankGameInstance` (`GameplayStatics.GetGameInstance`)))
  (set `self.GameInstance` _asbp_tank_game_instance)
  (return))

(fn `UserConstructionScript`)