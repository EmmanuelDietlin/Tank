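; Player controller for co-op tank multiplayer that handles each player's side of the lobby.
; It loads player info from the save game and passes it on, prompting the lobby game mode to update everyone.
; It creates the lobby menu and refreshes its map, game type and player list from incoming data.
; Being kicked or ending play destroys the session and, on success, opens the master level.
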(event `InitialSetup`
  (bind _returnvalue (`GameplayStatics.DoesSaveGameExist` "TankSave"))
  (if _returnvalue
    (bind _returnvalue_2 (`GameplayStatics.LoadGameFromSlot` "TankSave"))
    (bind _astank_save_game (cast `TankSaveGame` _returnvalue_2))
    (bind _output_get (set `self.Player Info` (`TankSaveGame.PlayerInfos` _astank_save_game)))
    (`self.CallUpdate` _output_get)))

(event `SetupLobbyMenu`
  (params (ServerName :type Text))
  (set `self.bShowMouseCursor` true)
  (bind _returnvalue (`|CreateWidget` "/Game/Tank/UI/WBP_LobbyMenu.WBP_LobbyMenu_C" null ServerName))
  (bind _output_get (set `self.LobbyMenu` _returnvalue))
  (`UserWidget.AddToViewport` _output_get 0)
  (`UserWidget.AddToViewport` _returnvalue 0)
  (`WidgetBlueprintLibrary.SetInputMode_GameAndUIEx` self _output_get))

(event `CallUpdate`
  (params (PlayerInfo :type "PlayerInfos Structure") (ChangedStatus :type Boolean))
  (set `self.Player Info` PlayerInfo)
  (bind _aslobby_game_mode (cast `/Game/Tank/Gameplay/LobbyGameMode` (`GameplayStatics.GetGameMode`)))
  (`/Game/Tank/Gameplay/LobbyGameMode.EveryoneUpdate` _aslobby_game_mode))

(event `UpdateLobbySettings`
  (params (MapName :type Text) (Gamemode :type Text))
  (bind _lobbymenu (`self.LobbyMenu`))
  (set `/Game/Tank/UI/WBP_LobbyMenu.MapName` MapName _lobbymenu)
  (set `/Game/Tank/UI/WBP_LobbyMenu.GameType` Gamemode _lobbymenu))

(event `AddPlayerInfo`
  (params (ConnectedPlayersInfos :type "Array of PlayerInfos Structure"))
  (bind _lobbymenu (`self.LobbyMenu`))
  (set `self.ConnectedPlayers` ConnectedPlayersInfos)
  (`/Engine/EditorBlueprintResources/StandardMacros.IsValid` _lobbymenu
    (:`Is Valid`
      (`/Game/Tank/UI/WBP_LobbyMenu.ClearPlayerList` _lobbymenu)
      (for _array_element (`self.ConnectedPlayers`)
        (`/Game/Tank/UI/WBP_LobbyMenu.UpdatePlayerWindow` (`self.LobbyMenu`) _array_element)))))

(event `self.ReceiveEndPlay`
  (params (EndPlayReason :type "EEndPlayReason Enum" :default "Destroyed"))
  (`DestroySessionCallbackProxy.DestroySession` self :!label _label
    (:`OnSuccess`
      (`GameplayStatics.OpenLevelBySoftObjectPtr` "/Game/Tank/Levels/LevelStreaming/MasterLevel.MasterLevel"))))

(event `Kicked`
  (goto _label))

(fn `UserConstructionScript`)