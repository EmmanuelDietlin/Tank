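; Player tank Blueprint that sets up the HUD and aims the turret at the mouse cursor.
; On BeginPlay it adds WBP_HUD to the viewport and shows the mouse cursor.
; Each Tick it traces under the cursor on the Visibility channel and, on a hit, turns TurretElement in world space toward that point, using only yaw so the turret stays level.
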(event `self.ReceiveBeginPlay`
  (bind _returnvalue (`|CreateWidget` "/Game/Tank/UI/WBP_HUD.WBP_HUD_C"))
  (`UserWidget.AddToViewport` _returnvalue 0)
  (set `PlayerController.bShowMouseCursor` true (`GameplayStatics.GetPlayerController` 0)))

(event `self.ReceiveTick`
  (params (DeltaSeconds :type "Float (single-precision)"))
  (bind _turretelement (`self.TurretElement`))
  (bind (_hitresult _returnvalue) (`PlayerController.GetHitResultUnderCursorByChannel` (`GameplayStatics.GetPlayerController` 0) "TraceTypeQuery1" true))
  (if _returnvalue
    (`SceneComponent.K2_SetWorldRotation` _turretelement (`KismetMathLibrary.MakeRotator` 0.0 0.0 (.yaw (`KismetMathLibrary.FindLookAtRotation` (`SceneComponent.K2_GetComponentLocation` _turretelement) (`.Location` (`GameplayStatics.BreakHitResult` _hitresult))))) false false)))

(fn `UserConstructionScript`)