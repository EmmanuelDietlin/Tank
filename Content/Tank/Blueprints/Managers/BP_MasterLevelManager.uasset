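; BP_MasterLevelManager is a level manager that puts the tank game into its main menu state on BeginPlay and whenever its OnMainMenu dispatcher fires.
; It tells BP_UIManager to show the menu and swaps the Enhanced Input mapping from tank controls to menu controls.
; It then calls TogglePause on BP_PlayerTank, first restarting the player through the GameMode if no tank exists.
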(event `self.ReceiveBeginPlay`
  (bind _returnvalue (pcsubsystem `EnhancedInputLocalPlayerSubsystem` (`GameplayStatics.GetPlayerController` 0)))
  (add `self.OnMainMenu` (delegate `OnMainMenu_Event`))
  (bind _returnvalue_2 (`GameplayStatics.GetActorOfClass` "/Game/Tank/UI/BP_UIManager.BP_UIManager_C" :!label _label))
  (`/Engine/EditorBlueprintResources/StandardMacros.IsValid` _returnvalue_2
    (:`Is Valid`
      (bind _output_get (set `self.UIManager` _returnvalue_2))
      (`/Game/Tank/UI/BP_UIManager.MainMenuUI` _output_get)
      (`/Engine/EditorBlueprintResources/StandardMacros.IsValid` _returnvalue
        (:`Is Valid`
          (`EnhancedInputSubsystemInterface.AddMappingContext` _returnvalue "/Game/Tank/Inputs/MainMenuInputMap.MainMenuInputMap" 0 (struct))
          (`EnhancedInputSubsystemInterface.RemoveMappingContext` _returnvalue "/Game/Tank/Inputs/TankInputMap.TankInputMap" (struct))
          (bind _returnvalue_3 (`GameplayStatics.GetActorOfClass` "/Game/Tank/Blueprints/Tanks/BP_PlayerTank.BP_PlayerTank_C"))
          (`/Engine/EditorBlueprintResources/StandardMacros.IsValid` _returnvalue_3
            (:`Is Valid`
              (`PlayerTank.TogglePause` _returnvalue_3 true))
            (:`Is Not Valid`
              (`GameModeBase.RestartPlayer` (`GameplayStatics.GetGameMode`) (`GameplayStatics.GetPlayerController` 0))
              (bind _returnvalue_4 (`GameplayStatics.GetActorOfClass` "/Game/Tank/Blueprints/Tanks/BP_PlayerTank.BP_PlayerTank_C"))
              (`PlayerTank.TogglePause` _returnvalue_4 true))))))))

(event `OnMainMenu_Event`
  (goto _label))

(fn `UserConstructionScript`)