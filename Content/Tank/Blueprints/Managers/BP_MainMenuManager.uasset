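; BP_MainMenuManager runs the tank game's main menu and the handoff into the first level.
; On BeginPlay it shows the menu through BP_UIManager, disables the player tank's tick, shows the cursor and swaps Enhanced Input to the menu mapping context.
; LoadFirstLevel restores tank input, then either passes the next-level UI to BP_MasterLevelManager for a delayed level change when streaming is enabled, or opens FirstLevel directly.
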(event `self.ReceiveBeginPlay`
  (bind _returnvalue (`GameplayStatics.GetPlayerController` 0))
  (bind _returnvalue_2 (pcsubsystem `EnhancedInputLocalPlayerSubsystem` _returnvalue))
  (bind _returnvalue_3 (`GameplayStatics.GetActorOfClass` "/Game/Tank/UI/BP_UIManager.BP_UIManager_C"))
  (`/Engine/EditorBlueprintResources/StandardMacros.IsValid` _returnvalue_3
    (:`Is Valid`
      (bind _output_get (set `self.UIManager` _returnvalue_3))
      (`/Game/Tank/UI/BP_UIManager.MainMenuUI` _output_get)
      (bind _returnvalue_4 (`GameplayStatics.GetActorOfClass` "/Game/Tank/Blueprints/Tanks/BP_PlayerTank.BP_PlayerTank_C"))
      (`/Engine/EditorBlueprintResources/StandardMacros.IsValid` _returnvalue_4
        (:`Is Valid`
          (`self.SetActorTickEnabled` _returnvalue_4 false)
          (set `PlayerController.bShowMouseCursor` true _returnvalue)
          (`/Engine/EditorBlueprintResources/StandardMacros.IsValid` _returnvalue_2
            (:`Is Valid`
              (`EnhancedInputSubsystemInterface.AddMappingContext` _returnvalue_2 "/Game/Tank/Inputs/MainMenuInputMap.MainMenuInputMap" 0 (struct))
              (`EnhancedInputSubsystemInterface.RemoveMappingContext` _returnvalue_2 "/Game/Tank/Inputs/TankInputMap.TankInputMap" (struct)))))))))

(event `LoadFirstLevel`
  (bind _returnvalue (pcsubsystem `EnhancedInputLocalPlayerSubsystem` (`GameplayStatics.GetPlayerController` 0)))
  (`EnhancedInputSubsystemInterface.AddMappingContext` _returnvalue "/Game/Tank/Inputs/TankInputMap.TankInputMap" 0 (struct))
  (`EnhancedInputSubsystemInterface.RemoveMappingContext` _returnvalue "/Game/Tank/Inputs/MainMenuInputMap.MainMenuInputMap" (struct))
  (if (`self.IsStreamingEnabled`)
    (`KismetSystemLibrary.DelayUntilNextTick`)
    (bind _fadeindelay (`/Game/Tank/UI/BP_UIManager.NextLevelUI` (`self.UIManager`)))
    (bind _returnvalue_2 (`GameplayStatics.GetActorOfClass` "/Game/Tank/Blueprints/Managers/BP_MasterLevelManager.BP_MasterLevelManager_C"))
    (`/Engine/EditorBlueprintResources/StandardMacros.IsValid` _returnvalue_2
      (:`Is Valid`
        (`MasterLevelManager.NextLevelWithDelay` _returnvalue_2 _fadeindelay)))
    (else
      (`GameplayStatics.OpenLevelBySoftObjectPtr` (`self.FirstLevel`)))))

(fn `UserConstructionScript`)