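; Level manager for the tank game that runs level start, pausing, player death and progression to victory or defeat screens.
; BeginPlay clears leftover weapons, snapshots the score and binds tank-destroyed events: enemy kills add score, while player death restores the snapshot and restarts if lives remain.
; The next-level delegate drives UIManager screens, whose destruct event triggers the level change.
; A LevelStreamingEnabled flag switches between BP_MasterLevelManager streaming and direct level loading.
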(event `OnNextLevel`
  (bind _uimanager (`self.UIManager`))
  (bind _tankgameinstance (`self.TankGameInstance`))
  (bind _outactors (`GameplayStatics.GetAllActorsWithTag` (`self.WeaponsTag`)))
  (for _array_element _outactors
    (`self.K2_DestroyActor` _array_element))
  (if (`self.LevelStreamingEnabled`)
    (bind _returnvalue (`GameplayStatics.GetActorOfClass` "/Game/Tank/Blueprints/Managers/BP_MasterLevelManager.BP_MasterLevelManager_C"))
    (`/Engine/EditorBlueprintResources/StandardMacros.IsValid` _returnvalue
      (:`Is Valid`
        (bind _returnvalue_2 (`MasterLevelManager.IsLastLevel` _returnvalue))
        (if _returnvalue_2
          (`/Game/Tank/UI/BP_UIManager.VictoryScreenUI` (`self.UIManager`) :!label _label)
          (`self.TogglePause` true)
          (else
            (set `TankGameInstance.LevelNumber` (+ (`TankGameInstance.LevelNumber` _tankgameinstance) 1) _tankgameinstance :!label _label_2)
            (`/Game/Tank/UI/BP_UIManager.LevelEndUI` _uimanager)
            (if (`self.LevelStreamingEnabled`)
              (add `/Game/Tank/UI/BP_UIManager.OnLevelEndDestruct` (`self.UIManager`) (delegate `OnLevelEndDestruct_streaming`))
              (else
                (add `/Game/Tank/UI/BP_UIManager.OnLevelEndDestruct` _uimanager (delegate `OnLevelEndDestruct_Event`))))
            (`self.TogglePause` true)))))
    (elif (`self.IsLastLevel`)
      (goto _label)
      (else
        (goto _label_2)))))

(event `OnLevelEndDestruct_Event`
  (`self.LoadNextLevel`))

(event `OnLevelEndDestruct_streaming`
  (bind _fadeindelay (`/Game/Tank/UI/BP_UIManager.NextLevelUI` (`self.UIManager`)))
  (`MasterLevelManager.NextLevelWithDelay` (stale `OnNextLevel` _returnvalue) _fadeindelay))

(event `self.ReceiveBeginPlay`
  (bind _returnvalue (`GameplayStatics.GetActorOfClass` "/Game/Tank/UI/BP_UIManager.BP_UIManager_C"))
  (set `self.UIManager` _returnvalue)
  (bind _astank_game_instance (cast `TankGameInstance` (`GameplayStatics.GetGameInstance`)))
  (bind _output_get (set `self.TankGameInstance` _astank_game_instance))
  (set `TankGameInstance.LevelScore` (`TankGameInstance.Score` _output_get) _output_get)
  (bind _outactors (`GameplayStatics.GetAllActorsWithTag` (`self.WeaponsTag`)))
  (for _array_element _outactors
    (`self.K2_DestroyActor` _array_element))
  (bind _outactors_2 (`GameplayStatics.GetAllActorsOfClass` "/Script/TanksGame.EnemyTank"))
  (for _array_element_2 _outactors_2
    (add `Tank.OnTankDestroyed` _array_element_2 (delegate `OnTankDestroyed_Event_2`)))
  (add `self.OnNextLevelDelegate` (delegate `OnNextLevel`))
  (bind _returnvalue_2 (`GameplayStatics.GetActorOfClass` "/Game/Tank/Blueprints/Tanks/BP_PlayerTank.BP_PlayerTank_C"))
  (add `Tank.OnTankDestroyed` _returnvalue_2 (delegate `OnTankDestroyed_Event_1`))
  (if (`self.LevelStreamingEnabled`)
    (`self.TogglePause` true)
    (bind _returnvalue_3 (`GameplayStatics.GetActorOfClass` "/Script/Engine.PlayerStart"))
    (`self.K2_SetActorLocation` _returnvalue_2 (`self.K2_GetActorLocation` _returnvalue_3) false true)
    (else
      (`/Game/Tank/UI/BP_UIManager.NextLevelUI` (`self.UIManager`))
      (`self.TogglePause` true))))

(event `OnTankDestroyed_Event_1`
  (`self.PlayerDeath`))

(event `OnTankDestroyed_Event_2`
  (bind _tankgameinstance (`self.TankGameInstance`))
  (set `TankGameInstance.Score` (+ (`TankGameInstance.Score` _tankgameinstance) 1) _tankgameinstance))

(event `PlayerDeath`
  (bind _returnvalue (`GameplayStatics.GetGameMode`))
  (bind _tankgameinstance (`self.TankGameInstance`))
  (`self.TogglePause` true)
  (bind _astank_game_instance (cast `TankGameInstance` (`GameplayStatics.GetGameInstance`)))
  (`/Engine/EditorBlueprintResources/StandardMacros.CompareInt` (`TankGameInstance.Lives` _astank_game_instance)
    (:`>`
      (`KismetSystemLibrary.Delay` 1.5)
      (set `TankGameInstance.Score` (`TankGameInstance.LevelScore` _tankgameinstance) _tankgameinstance)
      (if (`self.LevelStreamingEnabled`)
        (bind _fadeindelay (`/Game/Tank/UI/BP_UIManager.NextLevelUI` (`self.UIManager`)))
        (`KismetSystemLibrary.Delay` _fadeindelay)
        (`/Engine/EditorBlueprintResources/StandardMacros.IsValid` _returnvalue
          (:`Is Valid`
            (`GameModeBase.RestartPlayer` _returnvalue (`GameplayStatics.GetPlayerController` 0)))))
      (`self.RestartLevel`))
    (:`==`
      (`/Game/Tank/UI/BP_UIManager.DefeatScreenUI` (`self.UIManager`) :!label _label_3)
      (`self.TogglePause` true))
    (:`<`
      (goto _label_3))))

(event `Pause`
  (bind _ispausemenuvisible (`/Game/Tank/UI/BP_UIManager.TogglePauseMenu` (`self.UIManager`)))
  (`self.TogglePause` _ispausemenuvisible))

(fn `UserConstructionScript`)