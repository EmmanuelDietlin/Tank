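; Game instance for the tank game that owns menu flow, online sessions and persistent audio settings.
; Init loads sound and music volume from the TankSave slot and refills lives if a save exists, and Shutdown writes the volumes back.
; Show events clear all widgets and display menus or result screens, mostly cached, with the account menu replacing the main menu until a save exists.
; Session events host a listen-server lobby, join or destroy sessions.
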(event `self.ReceiveInit`
  (bind _returnvalue (`GameplayStatics.DoesSaveGameExist` "TankSave"))
  ;[1 1 1] Load game on game start and save game on game close
  (if _returnvalue
    (bind _returnvalue_2 (`GameplayStatics.LoadGameFromSlot` "TankSave"))
    (bind _astank_save_game (cast `TankSaveGame` _returnvalue_2))
    (set `self.SoundVolume` (`TankSaveGame.SoundVolume` _astank_save_game))
    (set `self.MusicVolume` (`TankSaveGame.MusicVolume` _astank_save_game))
    (set `self.Lives` (`self.MaxLives`))))

(event `self.ReceiveShutdown`
  ;[1 1 1] Load game on game start and save game on game close
  (bind _returnvalue (`GameplayStatics.LoadGameFromSlot` "TankSave"))
  (bind _astank_save_game (cast `TankSaveGame` _returnvalue))
  (set `TankSaveGame.SoundVolume` (`self.SoundVolume`) _astank_save_game)
  (set `TankSaveGame.MusicVolume` (`self.MusicVolume`) _astank_save_game)
  (`GameplayStatics.SaveGameToSlot` _astank_save_game "TankSave"))

(event `SessionDestroy`
  (params (PlayerController :type "PlayerController Object Reference"))
  (`DestroySessionCallbackProxy.DestroySession` PlayerController))

(event `ShowMainMenu`
  (bind _returnvalue (`GameplayStatics.GetPlayerController` 0))
  (bind _returnvalue_2 (`GameplayStatics.DoesSaveGameExist` "TankSave"))
  (if _returnvalue_2
    (`WidgetLayoutLibrary.RemoveAllWidgets`)
    (`/Engine/EditorBlueprintResources/StandardMacros.IsValid` (`self.MainMenuWB`)
      (:`Is Valid`
        _)
      (:`Is Not Valid`
        (bind _returnvalue_3 (`|CreateWidget` "/Game/Tank/UI/WBP_MainMenu.WBP_MainMenu_C" _returnvalue))
        (set `self.MainMenuWB` _returnvalue_3)))
    (`UserWidget.AddToViewport` (`self.MainMenuWB`) 0)
    (set `PlayerController.bShowMouseCursor` true _returnvalue)
    (else
      (`self.ShowAccountMenu`))))

(event `self.HandleTravelError`
  (params (FailureType :type "ETravelFailure Enum" :default "NoLevel"))
  (`KismetSystemLibrary.PrintString` (`|GetEnumeratorNameAsString` FailureType) true true (struct :`G` 0.66 :`B` 1.0 :`A` 1.0) 10.0))

(event `self.HandleNetworkError`
  (params (FailureType :type "ENetworkFailure Enum" :default "NetDriverAlreadyExists") (bIsServer :type Boolean))
  (`KismetSystemLibrary.PrintString` (`|GetEnumeratorNameAsString` FailureType) true true (struct :`G` 0.66 :`B` 1.0 :`A` 1.0) 10.0))

(event `ShowSettingsMenu`
  (`WidgetLayoutLibrary.RemoveAllWidgets`)
  (`/Engine/EditorBlueprintResources/StandardMacros.IsValid` (`self.SettingsMenu`)
    (:`Is Valid`
      _)
    (:`Is Not Valid`
      (bind _returnvalue (`|CreateWidget` "/Game/Tank/UI/WBP_SettingsMenu.WBP_SettingsMenu_C" (`GameplayStatics.GetPlayerController` 0)))
      (set `self.SettingsMenu` _returnvalue)))
  (`UserWidget.AddToViewport` (`self.SettingsMenu`) 0))

(event `LaunchLobby`
  (params (PlayersNumber :type Integer) (ServerName :type Text) (EnableLAN :type Boolean))
  (set `self.PlayersNumber` PlayersNumber)
  (set `self.ServerName` ServerName)
  (`CreateSessionCallbackProxy.CreateSession` (`GameplayStatics.GetPlayerController` 0) (`self.PlayersNumber`) EnableLAN
    (:`OnSuccess`
      (`GameplayStatics.OpenLevelBySoftObjectPtr` "/Game/Tank/Levels/LevelStreaming/StreamingLevelLobby.StreamingLevelLobby" true "listen"))
    (:`OnFailure`
      (`KismetSystemLibrary.PrintString` "Failed to create online session"))))

(event `ShowAccountMenu`
  (bind _returnvalue (`GameplayStatics.DoesSaveGameExist` "TankSave"))
  (if _returnvalue
    (`self.ShowMainMenu`)
    (else
      (`WidgetLayoutLibrary.RemoveAllWidgets`)
      (`/Engine/EditorBlueprintResources/StandardMacros.IsValid` (`self.AccountScreen`)
        (:`Is Valid`
          _)
        (:`Is Not Valid`
          (bind _returnvalue_2 (`|CreateWidget` "/Game/Tank/UI/WBP_AccountMenu.WBP_AccountMenu_C" (`GameplayStatics.GetPlayerController` 0)))
          (set `self.AccountScreen` _returnvalue_2)))
      (`UserWidget.AddToViewport` (`self.AccountScreen`) 0))))

(event `JoinServer`
  (params (SessionToJoin :type "BlueprintSessionResult Structure"))
  (`JoinSessionCallbackProxy.JoinSession` (`GameplayStatics.GetPlayerController` 0) SessionToJoin
    (:`OnSuccess`
      (`KismetSystemLibrary.PrintString` "Join session success"))
    (:`OnFailure`
      (`KismetSystemLibrary.PrintString` "Failed to join online session"))))

(event `ShowHostMenu`
  (`WidgetLayoutLibrary.RemoveAllWidgets`)
  (`/Engine/EditorBlueprintResources/StandardMacros.IsValid` (`self.HostMenu`)
    (:`Is Valid`
      _)
    (:`Is Not Valid`
      (bind _returnvalue (`|CreateWidget` "/Game/Tank/UI/WBP_HostMenu.WBP_HostMenu_C" (`GameplayStatics.GetPlayerController` 0)))
      (set `self.HostMenu` _returnvalue)))
  (`UserWidget.AddToViewport` (`self.HostMenu`) 0))

(event `ShowJoinMenu`
  (`WidgetLayoutLibrary.RemoveAllWidgets`)
  (`/Engine/EditorBlueprintResources/StandardMacros.IsValid` (`self.ServerMenu`)
    (:`Is Valid`
      _)
    (:`Is Not Valid`
      (bind _returnvalue (`|CreateWidget` "/Game/Tank/UI/WBP_ServerMenu.WBP_ServerMenu_C" (`GameplayStatics.GetPlayerController` 0)))
      (set `self.ServerMenu` _returnvalue)))
  (`UserWidget.AddToViewport` (`self.ServerMenu`) 0))

(event `ShowVictoryScreen`
  (`WidgetLayoutLibrary.RemoveAllWidgets`)
  (`/Engine/EditorBlueprintResources/StandardMacros.IsValid` (`self.VictoryScreen`)
    (:`Is Valid`
      _)
    (:`Is Not Valid`
      (bind _returnvalue (`|CreateWidget` "/Game/Tank/UI/WBP_VictoryScreen_.WBP_VictoryScreen__C" (`GameplayStatics.GetPlayerController` 0)))
      (set `self.VictoryScreen` _returnvalue)))
  (`UserWidget.AddToViewport` (`self.VictoryScreen`) 0))

(event `ShowDefeatScreen`
  (`WidgetLayoutLibrary.RemoveAllWidgets`)
  (`/Engine/EditorBlueprintResources/StandardMacros.IsValid` (`self.DefeatScreen`)
    (:`Is Valid`
      _)
    (:`Is Not Valid`
      (bind _returnvalue (`|CreateWidget` "/Game/Tank/UI/WBP_DefeatScreen_.WBP_DefeatScreen__C" (`GameplayStatics.GetPlayerController` 0)))
      (set `self.DefeatScreen` _returnvalue)))
  (`UserWidget.AddToViewport` (`self.DefeatScreen`) 0))

(event `ShowLevelEndScreen`
  (`WidgetLayoutLibrary.RemoveAllWidgets`)
  (bind _returnvalue (`|CreateWidget` "/Game/Tank/UI/WBP_LevelEndScreen.WBP_LevelEndScreen_C" (`GameplayStatics.GetPlayerController` 0)))
  (`UserWidget.AddToViewport` _returnvalue 0))

(event `ShowNextLevelScreen`
  (`WidgetLayoutLibrary.RemoveAllWidgets`)
  (`self.HUD`)
  (`self.TransitionScreen`))

(fn `HUD`
  (bind _returnvalue (`|CreateWidget` "/Game/Tank/UI/WBP_HUD.WBP_HUD_C" (`GameplayStatics.GetPlayerController` 0)))
  (`UserWidget.AddToViewport` _returnvalue 0))

(fn `TransitionScreen`
  (returns (BackgroundFadeInTime :type "Float (double-precision)"))
  (bind _returnvalue (`|CreateWidget` "/Game/Tank/UI/WBP_TransitionScreen.WBP_TransitionScreen_C" (`GameplayStatics.GetPlayerController` 0)))
  (`UserWidget.AddToViewport` _returnvalue 0)
  (return (`/Game/Tank/UI/WBP_TransitionScreen.BackgroundFadeInTime` _returnvalue)))