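; Player tank pawn Blueprint that links itself to the level's enemy tanks and handles its own destruction.
; On BeginPlay it sets itself as every EnemyTank's target reference, shows the mouse cursor, caches the level manager and prints the level name.
; When destroyed, it decrements Lives in the TankGameInstance and spawns Mine_Particles at its transform.
; Pause logic through the level manager exists but is disconnected from the empty Tank_Pause input event.
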(event `self.ReceiveBeginPlay`
  (bind _outactors (`GameplayStatics.GetAllActorsOfClass` "/Script/TanksGame.EnemyTank"))
  (for _array_element _outactors
    (set `EnemyTank.PlayerTank` self _array_element))
  (set `PlayerController.bShowMouseCursor` true (`GameplayStatics.GetPlayerController` 0))
  (bind _returnvalue (`GameplayStatics.GetActorOfClass` "/Game/Tank/Blueprints/Managers/BP_LevelManager.BP_LevelManager_C"))
  (set `self.LevelManager` _returnvalue)
  (add `Tank.OnTankDestroyed` (delegate `OnTankDestroyed_Event_0`))
  (bind _returnvalue_2 (`GameplayStatics.GetCurrentLevelName` true))
  (`KismetSystemLibrary.PrintString` _returnvalue_2))

(event `OnTankDestroyed_Event_0`
  (bind _astank_game_instance (cast `TankGameInstance` (`GameplayStatics.GetGameInstance`)))
  (set `TankGameInstance.Lives` (- (`TankGameInstance.Lives` _astank_game_instance) 1) _astank_game_instance)
  (`|SpawnActorFromClass` "/Game/Tank/Blueprints/Weapons/Mine_Particles.Mine_Particles_C" (`self.GetTransform`) "Undefined" "MultiplyWithRoot" null null))

(event `self.ReceiveTick`
  (params (DeltaSeconds :type "Float (single-precision)")))

(event `EnhancedInput|/Game/Tank/Inputs/Tank_Pause`
  (params (ActionValue :type Boolean) (ElapsedSeconds :type "Float (double-precision)") (TriggeredSeconds :type "Float (double-precision)") (InputAction :type "InputAction Object Reference" :default "/Game/Tank/Inputs/Tank_Pause.Tank_Pause")))

(fn `UserConstructionScript`)