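; BP_Mine is a tank weapon mine that detonates when an enemy tank enters its trigger sphere.
; On sphere overlap, it checks the tank's actor tags against EnemyTags and, for each match, calls TakeHit on the tank and Explode on itself.
; A destroy handler bound at BeginPlay spawns Mine_Particles at the mine's transform whenever it is destroyed.
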(event `self.ReceiveBeginPlay`
  (add `self.OnDestroyed` (delegate `Destroy`)))

(event `Destroy` :!signature `self.OnDestroyed`
  (params (DestroyedActor :type "Actor Object Reference"))
  (`|SpawnActorFromClass` "/Game/Tank/Blueprints/Weapons/Mine_Particles.Mine_Particles_C" (`self.GetTransform`) "Undefined" "MultiplyWithRoot" null null))

(event `self.Sphere.OnComponentBeginOverlap`
  (params (OverlappedComponent :type "PrimitiveComponent Object Reference") (OtherActor :type "Actor Object Reference") (OtherComp :type "PrimitiveComponent Object Reference") (OtherBodyIndex :type Integer) (bFromSweep :type Boolean) (SweepResult :type "HitResult Structure (by ref)"))
  (bind _astank (cast `Tank` OtherActor))
  (for _array_element (`self.EnemyTags`)
    (if (`self.ActorHasTag` _astank (`KismetStringLibrary.Conv_StringToName` _array_element))
      (`Tank.TakeHit` _astank)
      (`self.Explode`))))

(fn `UserConstructionScript`)