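; BP_EnemyMine is a tank-game mine that explodes on contact with a Tank or Projectile.
; Contact detonation arms once a Tank leaves the capsule, so a tank overlapping at spawn does not trigger it.
; On the authority, an overlap while explosion is allowed calls Explode and TakeHit on each gathered target, destroying any triggering projectile first.
; Its OnDestroyed binding spawns Mine_Particles at the mine's transform.
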(event `self.ReceiveBeginPlay`
  (set `self.CanExplodeOnContact` false)
  (add `self.OnDestroyed` (delegate `Destroy`)))

(event `Destroy` :!signature `self.OnDestroyed`
  (params (DestroyedActor :type "Actor Object Reference"))
  (`|SpawnActorFromClass` "/Game/Tank/Blueprints/Weapons/Mine_Particles.Mine_Particles_C" (`self.GetTransform`) "Undefined" "MultiplyWithRoot" null null))

(event `self.Capsule.OnComponentEndOverlap`
  (params (OverlappedComponent :type "PrimitiveComponent Object Reference") (OtherActor :type "Actor Object Reference") (OtherComp :type "PrimitiveComponent Object Reference") (OtherBodyIndex :type Integer))
  (cast `Tank` OtherActor)
  (set `self.CanExplodeOnContact` true))

(event `self.Capsule.OnComponentBeginOverlap`
  (params (OverlappedComponent :type "PrimitiveComponent Object Reference") (OtherActor :type "Actor Object Reference") (OtherComp :type "PrimitiveComponent Object Reference") (OtherBodyIndex :type Integer) (bFromSweep :type Boolean) (SweepResult :type "HitResult Structure (by ref)"))
  (if (`|EnumEquality` (`self.GetLocalRole`) "ROLE_Authority")
    (if (`self.CanExplode`)
      (if (`self.CanExplodeOnContact`)
        (cast `Tank` OtherActor
          (:`then`
            _)
          (:`CastFailed`
            (bind _asprojectile (cast `Projectile` OtherActor))
            (`self.K2_DestroyActor` _asprojectile)))
        (`self.Explode`)
        (for _array_element _
          (`Tank.TakeHit` _array_element))))))

(fn `UserConstructionScript`)