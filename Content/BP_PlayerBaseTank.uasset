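; Player tank base Blueprint that rotates its turret to face the mouse cursor.
; BeginPlay shows the cursor, then each Tick traces under it on the Camera channel and stores the hit location in MousePos.
; On a hit, the turret turns toward that point at a constant TurretRotationSpeed, keeping only world yaw so pitch and roll stay zero.
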(event `self.ReceiveBeginPlay`
  (set `PlayerController.bShowMouseCursor` true (`GameplayStatics.GetPlayerController` 0)))

(event `self.ReceiveTick`
  (params (DeltaSeconds :type "Float (single-precision)"))
  (bind _mousepos (`self.MousePos`))
  (bind (_hitresult _returnvalue) (`PlayerController.GetHitResultUnderCursorByChannel` (`GameplayStatics.GetPlayerController` 0) "TraceTypeQuery2" true))
  (bind (_bblockinghit _binitialoverlap _time _distance _location) (`GameplayStatics.BreakHitResult` _hitresult))
  (if _returnvalue
    (if (`KismetMathLibrary.NotEqualExactly_VectorVector` _mousepos _location)
      (set `self.MousePos` _location))
    (`SceneComponent.K2_SetWorldRotation` (`self.TurretElement`) (`KismetMathLibrary.MakeRotator` 0.0 0.0 (.yaw (`KismetMathLibrary.RInterpTo_Constant` (`SceneComponent.K2_GetComponentRotation` (`self.TurretElement`)) (`KismetMathLibrary.FindLookAtRotation` (`SceneComponent.K2_GetComponentLocation` (`self.TurretElement`)) _mousepos) DeltaSeconds (`self.TurretRotationSpeed`)))) false false)))

(fn `UserConstructionScript`)