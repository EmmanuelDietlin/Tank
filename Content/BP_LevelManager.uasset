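; BP_LevelManager is the level manager that handles the end of play by showing a victory or defeat screen.
; On BeginPlay it binds OnPlayerVictory to the victory delegate, while PlayerDeath is a separate event with no caller in this graph.
; Both events remove all widgets, create their screen widget for the first player controller, add it to the player screen and pause the game.
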(event `self.ReceiveBeginPlay`
  (add `self.OnVictoryDelegate` (delegate `OnPlayerVictory`)))

(event `OnPlayerVictory`
  (`WidgetLayoutLibrary.RemoveAllWidgets`)
  (bind _returnvalue (`|CreateWidget` "/Game/Tank/UI/WBP_VictoryScreen.WBP_VictoryScreen_C" (`GameplayStatics.GetPlayerController` 0)))
  (`UserWidget.AddToPlayerScreen` _returnvalue 0)
  (`GameplayStatics.SetGamePaused` true))

(event `PlayerDeath`
  (`WidgetLayoutLibrary.RemoveAllWidgets`)
  (bind _returnvalue (`|CreateWidget` "/Game/Tank/UI/WBP_DefeatScreen.WBP_DefeatScreen_C" (`GameplayStatics.GetPlayerController` 0)))
  (`UserWidget.AddToPlayerScreen` _returnvalue 0)
  (`GameplayStatics.SetGamePaused` true))

(fn `UserConstructionScript`)